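; Player Blueprint for an infinite runner, Rosales, that manages its main HUD and its reaction to defeat.
; BeginPlay creates the main widget, stores it and adds it to the viewport.
; On defeat, SetUpPlayer stops running and moves the player to a hard-coded transform.
; If a MatchScoreCamera exists, the view blends to it, the defeated flag is set and the widget shows a loss.
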(event `self.ReceiveBeginPlay`
  (bind _returnvalue (`|CreateWidget` "/Game/Blueprints/UMG/MainWidget_BP.MainWidget_BP_C"))
  (`self.SetMainWidget` _returnvalue)
  (bind _returnvalue_2 (`self.GetMainWidget`))
  (`UserWidget.AddToViewport` _returnvalue_2 0))

(event `self.OnDefeatedEvent`
  (`self.SetUpPlayer`)
  (bind _returnvalue (`GameplayStatics.GetActorOfClass` "/Script/InfiniteRunner.MatchScoreCamera"))
  (`/Engine/EditorBlueprintResources/StandardMacros.IsValid` _returnvalue
    (:`Is Valid`
      (bind _output_get (set `self.MatchScoreCamera` _returnvalue))
      (`PlayerController.SetViewTargetWithBlend` (`GameplayStatics.GetPlayerController` 0) _output_get 4.0 "VTBlend_Linear" 20.0 false)
      (`self.SetIsDefeated` true)
      (bind _returnvalue_2 (`self.GetMainWidget`))
      (`MainWidget.SetMatchScoreTextBlock` _returnvalue_2 "Lost"))))

(fn `SetUpPlayer`
  (`self.SetIsRunning` false)
  (`self.K2_SetActorTransform` (`KismetMathLibrary.MakeTransform` (418.563751 4000.52832 -250.991394) (struct :`Yaw` 180.0))))

(fn `UserConstructionScript`)